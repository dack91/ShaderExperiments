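; BP_Rust is a shader test actor that toggles a rust effect when the player presses R.
; It enables input for the first player controller on BeginPlay and tracks the current state in an IsRusted flag.
; Each press plays or reverses a timeline whose tracks drive normal blend, opacity and world blend parameters in the MPC_Rust material parameter collection, animating the transition both ways.
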(event `self.ReceiveBeginPlay`
  (`self.EnableInput` (`GameplayStatics.GetPlayerController` 0)))

(event `Key|R`
  (params (Key :type "Key Structure" :default "AnyKey"))
  (:`Pressed`
    (if (`self.isRusted`)
      (set `self.isRusted` false)
      (bind (_direction _bn _op _wbm) (`Timeline|Timeline_0` :!via `Reverse` :!label _label)
        (:`Update`
          (`KismetMaterialLibrary.SetScalarParameterValue` "/Game/ShaderTests/OldMossSnowBlends/MPC_Rust.MPC_Rust" "BlendNormal" _bn)
          (`KismetMaterialLibrary.SetScalarParameterValue` "/Game/ShaderTests/OldMossSnowBlends/MPC_Rust.MPC_Rust" "Opacity" _op)
          (`KismetMaterialLibrary.SetScalarParameterValue` "/Game/ShaderTests/OldMossSnowBlends/MPC_Rust.MPC_Rust" "WorldBlendMax" _wbm)))
      (else
        (set `self.isRusted` true)
        (goto _label)))))

(fn `UserConstructionScript`)