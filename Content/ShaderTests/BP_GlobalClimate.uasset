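; BP_GlobalClimate is an actor in the shader tests that toggles world-wide rust and moss/snow material effects at runtime.
; It enables player input on BeginPlay, and E key handlers flip the IsRusted and IsWinter flags, playing or reversing a timeline for each.
; The timelines write blend, opacity and roughness values into MPC_Rust and MPC_MossSnowCycle, so materials reading those parameter collections transition together.
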(event `self.ReceiveBeginPlay`
  ;[1 1 1] Enable INput
  (`self.EnableInput` (`GameplayStatics.GetPlayerController` 0)))

(event `Key|E` :consume false
  (params (Key :type "Key Structure" :default "AnyKey"))
  ;[1 1 1] Rust
  (:`Pressed`
    (if (`self.isRusted`)
      (set `self.isRusted` false)
      (bind (_direction _bn _op _wbm) (`Timeline|Timeline_0` :!via `Reverse` :!label _label)
        (:`Update`
          (`KismetMaterialLibrary.SetScalarParameterValue` "/Game/ShaderTests/MPC_Rust.MPC_Rust" "BlendNormal" _bn)
          (`KismetMaterialLibrary.SetScalarParameterValue` "/Game/ShaderTests/MPC_Rust.MPC_Rust" "Opacity" _op)
          (`KismetMaterialLibrary.SetScalarParameterValue` "/Game/ShaderTests/MPC_Rust.MPC_Rust" "WorldBlendMax" _wbm)))
      (else
        (set `self.isRusted` true)
        (goto _label)))))

(event `Key|E` :consume false
  (params (Key :type "Key Structure" :default "AnyKey"))
  ;[1 1 1] Moss and Snow
  (:`Pressed`
    (if (`self.isWinter`)
      (set `self.isWinter` false)
      (bind (_direction _mossvsnow_value _opacity_value _roughness_value _blendnormal _worldblendmax) (`Timeline|Timeline_1` :!via `Reverse` :!label _label_2)
        (:`Update`
          (`KismetMaterialLibrary.SetScalarParameterValue` "/Game/ShaderTests/MPC_MossSnowCycle.MPC_MossSnowCycle" "MossVSnow" _mossvsnow_value)
          (`KismetMaterialLibrary.SetScalarParameterValue` "/Game/ShaderTests/MPC_MossSnowCycle.MPC_MossSnowCycle" "Opacity" _opacity_value)
          (`KismetMaterialLibrary.SetScalarParameterValue` "/Game/ShaderTests/MPC_MossSnowCycle.MPC_MossSnowCycle" "Roughness" _roughness_value)
          (`KismetMaterialLibrary.SetScalarParameterValue` "/Game/ShaderTests/MPC_MossSnowCycle.MPC_MossSnowCycle" "BlendNormal" _blendnormal)
          (`KismetMaterialLibrary.SetScalarParameterValue` "/Game/ShaderTests/MPC_MossSnowCycle.MPC_MossSnowCycle" "WorldBlendMax" _worldblendmax)))
      (else
        (set `self.isWinter` true)
        (goto _label_2)))))

(fn `UserConstructionScript`)